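; BP_Door is a door actor that slides its mesh from a closed to an open position.
; Tick polls the IsOpen flag and, through a DoOnce, calls Open a single time.
; Open plays the OpenDoor timeline, whose track lerps the DoorMesh relative location between ClosedLocation and OpenLocation.
; The file contains no closing logic and does not set IsOpen itself.
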(event `Open`
  (bind (_direction _opendoor) (`Timeline|OpenDoor` :!via `PlayFromStart`)
    (:`Update`
      (`SceneComponent.K2_SetRelativeLocation` (`self.DoorMesh`) (`KismetMathLibrary.VLerp` (`self.ClosedLocation`) (`self.OpenLocation`) _opendoor) false false))))

(event `self.ReceiveTick`
  (params (DeltaSeconds :type "Float (single-precision)"))
  (if (`self.IsOpen`)
    (`/Engine/EditorBlueprintResources/StandardMacros.DoOnce` false
      (:`Completed`
        (`self.Open`)))))

(fn `UserConstructionScript`)